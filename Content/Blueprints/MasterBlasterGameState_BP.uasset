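; MasterBlasterGameState_BP is a game state Blueprint that alternates turns between the player and the AI enemy.
; UpdateGameState checks whose turn it is and runs that side's turn update.
; When the update returns true, it hands over to the other side through BeginAITurn or BeginPlayerTurn, which each wait briefly before calling BeginEnemyTurn or BeginPlayerTurn.
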(event Custom|Update%20Game%20State
  (bind _returnvalue (Class|MasterBlasterGameState|GetIsPlayerTurn))
  (if _returnvalue
    (bind _returnvalue_2 (Class|MasterBlasterGameState|PlayerTurnUpdate))
    (if _returnvalue_2
      (CallFunction|BeginAITUrn))
    (else
      (bind _returnvalue_3 (Class|MasterBlasterGameState|EnemyTurnUpdate))
      (if _returnvalue_3
        (CallFunction|BeginPlayerTurn)))))

(event Custom|Begin%20AI%20Turn
  (Utilities|FlowControl|Delay 1.0)
  (Class|MasterBlasterGameState|BeginEnemyTurn))

(event Custom|Begin%20Player%20Turn
  (Utilities|FlowControl|Delay 1.0)
  (Class|MasterBlasterGameState|BeginPlayerTurn))

(fn ConstructionScript)