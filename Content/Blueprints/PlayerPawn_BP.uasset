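; Player pawn that moves through the level within bounds, driven by pan left/right, pan up/down and zoom axis inputs.
; All three inputs share one chain that scales axis values by speed and frame delta time, adds them to the actor location and sets it without sweeping.
; X and Y clamp to fixed ranges, while the symmetric Z limit narrows linearly as Y increases, tying vertical range to depth.
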(event Input|AxisEvents|InputAxisPanL_R
  (params (AxisValue :type Float%20%28single-precision%29))
  (bind _returnvalue (Utilities|Time|GetWorldDeltaSeconds))
  ;[1 1 1] Input * Duration
  (Transformation|SetActorLocation (Math|Vector|MakeVector (Math|Float|Clamp(Float) (.X (Math|Vector|BreakVector (+ (Math|Vector|MakeVector (* (* AxisValue (Variables|Default|GetSpeed)) _returnvalue) (* (* (stale Input|AxisEvents|InputAxisZoom AxisValue) (Variables|Default|GetSpeed)) _returnvalue) (* _returnvalue (* (stale Input|AxisEvents|InputAxisPanU_D AxisValue) (Variables|Default|GetSpeed)))) (Transformation|GetActorLocation)))) 0.0 4e+04) (Math|Float|Clamp(Float) (.Y (Math|Vector|BreakVector (+ (Math|Vector|MakeVector (* (* AxisValue (Variables|Default|GetSpeed)) _returnvalue) (* (* (stale Input|AxisEvents|InputAxisZoom AxisValue) (Variables|Default|GetSpeed)) _returnvalue) (* _returnvalue (* (stale Input|AxisEvents|InputAxisPanU_D AxisValue) (Variables|Default|GetSpeed)))) (Transformation|GetActorLocation)))) 1e+03 8e+03) (Math|Float|Clamp(Float) (.Z (Math|Vector|BreakVector (+ (Math|Vector|MakeVector (* (* AxisValue (Variables|Default|GetSpeed)) _returnvalue) (* (* (stale Input|AxisEvents|InputAxisZoom AxisValue) (Variables|Default|GetSpeed)) _returnvalue) (* _returnvalue (* (stale Input|AxisEvents|InputAxisPanU_D AxisValue) (Variables|Default|GetSpeed)))) (Transformation|GetActorLocation)))) (* (- 4e+03 (* (Math|Float|Clamp(Float) (.Y (Math|Vector|BreakVector (+ (Math|Vector|MakeVector (* (* AxisValue (Variables|Default|GetSpeed)) _returnvalue) (* (* (stale Input|AxisEvents|InputAxisZoom AxisValue) (Variables|Default|GetSpeed)) _returnvalue) (* _returnvalue (* (stale Input|AxisEvents|InputAxisPanU_D AxisValue) (Variables|Default|GetSpeed)))) (Transformation|GetActorLocation)))) 1e+03 8e+03) 0.5)) -1.0) (- 4e+03 (* (Math|Float|Clamp(Float) (.Y (Math|Vector|BreakVector (+ (Math|Vector|MakeVector (* (* AxisValue (Variables|Default|GetSpeed)) _returnvalue) (* (* (stale Input|AxisEvents|InputAxisZoom AxisValue) (Variables|Default|GetSpeed)) _returnvalue) (* _returnvalue (* (stale Input|AxisEvents|InputAxisPanU_D AxisValue) (Variables|Default|GetSpeed)))) (Transformation|GetActorLocation)))) 1e+03 8e+03) 0.5)))) false false))

(event Input|AxisEvents|InputAxisPanU_D
  (params (AxisValue :type Float%20%28single-precision%29))
  (bind _returnvalue (Utilities|Time|GetWorldDeltaSeconds))
  ;[1 1 1] Input * Duration
  (Transformation|SetActorLocation (Math|Vector|MakeVector (Math|Float|Clamp(Float) (.X (Math|Vector|BreakVector (+ (Math|Vector|MakeVector (* (* (stale Input|AxisEvents|InputAxisPanL_R AxisValue) (Variables|Default|GetSpeed)) _returnvalue) (* (* (stale Input|AxisEvents|InputAxisZoom AxisValue) (Variables|Default|GetSpeed)) _returnvalue) (* _returnvalue (* AxisValue (Variables|Default|GetSpeed)))) (Transformation|GetActorLocation)))) 0.0 4e+04) (Math|Float|Clamp(Float) (.Y (Math|Vector|BreakVector (+ (Math|Vector|MakeVector (* (* (stale Input|AxisEvents|InputAxisPanL_R AxisValue) (Variables|Default|GetSpeed)) _returnvalue) (* (* (stale Input|AxisEvents|InputAxisZoom AxisValue) (Variables|Default|GetSpeed)) _returnvalue) (* _returnvalue (* AxisValue (Variables|Default|GetSpeed)))) (Transformation|GetActorLocation)))) 1e+03 8e+03) (Math|Float|Clamp(Float) (.Z (Math|Vector|BreakVector (+ (Math|Vector|MakeVector (* (* (stale Input|AxisEvents|InputAxisPanL_R AxisValue) (Variables|Default|GetSpeed)) _returnvalue) (* (* (stale Input|AxisEvents|InputAxisZoom AxisValue) (Variables|Default|GetSpeed)) _returnvalue) (* _returnvalue (* AxisValue (Variables|Default|GetSpeed)))) (Transformation|GetActorLocation)))) (* (- 4e+03 (* (Math|Float|Clamp(Float) (.Y (Math|Vector|BreakVector (+ (Math|Vector|MakeVector (* (* (stale Input|AxisEvents|InputAxisPanL_R AxisValue) (Variables|Default|GetSpeed)) _returnvalue) (* (* (stale Input|AxisEvents|InputAxisZoom AxisValue) (Variables|Default|GetSpeed)) _returnvalue) (* _returnvalue (* AxisValue (Variables|Default|GetSpeed)))) (Transformation|GetActorLocation)))) 1e+03 8e+03) 0.5)) -1.0) (- 4e+03 (* (Math|Float|Clamp(Float) (.Y (Math|Vector|BreakVector (+ (Math|Vector|MakeVector (* (* (stale Input|AxisEvents|InputAxisPanL_R AxisValue) (Variables|Default|GetSpeed)) _returnvalue) (* (* (stale Input|AxisEvents|InputAxisZoom AxisValue) (Variables|Default|GetSpeed)) _returnvalue) (* _returnvalue (* AxisValue (Variables|Default|GetSpeed)))) (Transformation|GetActorLocation)))) 1e+03 8e+03) 0.5)))) false false))

(event Input|AxisEvents|InputAxisZoom
  (params (AxisValue :type Float%20%28single-precision%29))
  (bind _returnvalue (Utilities|Time|GetWorldDeltaSeconds))
  ;[1 1 1] Input * Duration
  (Transformation|SetActorLocation (Math|Vector|MakeVector (Math|Float|Clamp(Float) (.X (Math|Vector|BreakVector (+ (Math|Vector|MakeVector (* (* (stale Input|AxisEvents|InputAxisPanL_R AxisValue) (Variables|Default|GetSpeed)) _returnvalue) (* (* AxisValue (Variables|Default|GetSpeed)) _returnvalue) (* _returnvalue (* (stale Input|AxisEvents|InputAxisPanU_D AxisValue) (Variables|Default|GetSpeed)))) (Transformation|GetActorLocation)))) 0.0 4e+04) (Math|Float|Clamp(Float) (.Y (Math|Vector|BreakVector (+ (Math|Vector|MakeVector (* (* (stale Input|AxisEvents|InputAxisPanL_R AxisValue) (Variables|Default|GetSpeed)) _returnvalue) (* (* AxisValue (Variables|Default|GetSpeed)) _returnvalue) (* _returnvalue (* (stale Input|AxisEvents|InputAxisPanU_D AxisValue) (Variables|Default|GetSpeed)))) (Transformation|GetActorLocation)))) 1e+03 8e+03) (Math|Float|Clamp(Float) (.Z (Math|Vector|BreakVector (+ (Math|Vector|MakeVector (* (* (stale Input|AxisEvents|InputAxisPanL_R AxisValue) (Variables|Default|GetSpeed)) _returnvalue) (* (* AxisValue (Variables|Default|GetSpeed)) _returnvalue) (* _returnvalue (* (stale Input|AxisEvents|InputAxisPanU_D AxisValue) (Variables|Default|GetSpeed)))) (Transformation|GetActorLocation)))) (* (- 4e+03 (* (Math|Float|Clamp(Float) (.Y (Math|Vector|BreakVector (+ (Math|Vector|MakeVector (* (* (stale Input|AxisEvents|InputAxisPanL_R AxisValue) (Variables|Default|GetSpeed)) _returnvalue) (* (* AxisValue (Variables|Default|GetSpeed)) _returnvalue) (* _returnvalue (* (stale Input|AxisEvents|InputAxisPanU_D AxisValue) (Variables|Default|GetSpeed)))) (Transformation|GetActorLocation)))) 1e+03 8e+03) 0.5)) -1.0) (- 4e+03 (* (Math|Float|Clamp(Float) (.Y (Math|Vector|BreakVector (+ (Math|Vector|MakeVector (* (* (stale Input|AxisEvents|InputAxisPanL_R AxisValue) (Variables|Default|GetSpeed)) _returnvalue) (* (* AxisValue (Variables|Default|GetSpeed)) _returnvalue) (* _returnvalue (* (stale Input|AxisEvents|InputAxisPanU_D AxisValue) (Variables|Default|GetSpeed)))) (Transformation|GetActorLocation)))) 1e+03 8e+03) 0.5)))) false false))

(fn ConstructionScript)