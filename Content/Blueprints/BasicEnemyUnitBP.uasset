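; BasicEnemyUnitBP is a basic enemy unit Blueprint built on a Paper2D flipbook sprite with a separate arm component.
; On BeginPlay it attaches the Arm to the sprite's GunArm socket, keeping relative transforms.
; Each Tick calls UpdateAnimation, which sets the enemy idle flipbook only when the unit is moving, with no other animation branch.
; A disconnected node referencing the player unit's idle flipbook never runs.
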(event Custom|UpdateAnimation
  (bind _returnvalue (Class|BaseUnit|GetIsMoving))
  (if _returnvalue
    (Sprite|SetFlipbook (Variables|Default|GetSprite) "/Game/Sprites/EnemySprites/Idle/EnemyIdleAnimation.EnemyIdleAnimation")))

(event EventBeginPlay
  (Transformation|AttachComponentToComponent (Variables|Default|GetArm) (Variables|Default|GetSprite) "GunArm" "KeepRelative" "KeepRelative" "KeepRelative" true))

(event EventTick
  (params (DeltaSeconds :type Float%20%28single-precision%29))
  (CallFunction|UpdateAnimation))

(fn ConstructionScript)