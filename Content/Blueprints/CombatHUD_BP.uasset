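; Combat HUD Blueprint that shows the player the objective of destroying all enemy units and how many enemies remain.
; On each DrawHUD event it draws both lines with DrawText in a scribbly font.
; The remaining count is read directly from the length of the EnemyTeam array on MasterBlasterGameState, so that line is skipped if the game state cast fails.
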(event EventDrawHUD
  (params (SizeX :type Integer) (SizeY :type Integer))
  (HUD|DrawText (Utilities|String|ToString(Text) (Utilities|Text|MakeLiteralText "Objective: Destroy All Enemy Units")) "(R=0.000000,G=0.000000,B=0.000000,A=1.000000)" 0.0 0.0 "/Game/Materials/Fonts/ScribblyFont_Font.ScribblyFont_Font" 1.0 false)
  (bind _asmaster_blaster_game_state (Utilities|Casting|CastToMasterBlasterGameState (Game|GetGameState)))
  (HUD|DrawText (Utilities|String|Append (Utilities|String|MakeLiteralString "Enemies Remaining: ") (Utilities|String|ToString(Text) (Utilities|Text|ToText(String) (Utilities|String|ToString(Integer) (Utilities|Array|Length (Variables|/Script/MasterBlaster.MasterBlasterGameState|GetEnemyTeam _asmaster_blaster_game_state)))))) "(R=0,G=0,B=0,A=1)" 0.0 3e+01 "/Game/Materials/Fonts/ScribblyFont_Font.ScribblyFont_Font" 0.75 false))

(fn ConstructionScript)