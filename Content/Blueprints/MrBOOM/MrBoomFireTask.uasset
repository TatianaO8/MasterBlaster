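; Behavior tree task that makes the AI-controlled MrBoom fire a six-shell cannon burst.
; It flags the pawn as fired, plays the open-fire sound, then runs a macro that spawns MrBoomShell actors separated by short fixed delays.
; Each shell spawns at the cannon's Muzzle socket, using the cannon's world rotation with pitch flipped 180 degrees.
; Afterwards it clears the Target blackboard value and finishes as failed.
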(event EventReceiveExecute
  (params (OwnerActor :type Actor%20Object%20Reference))
  (bind _asmr_boom_aicontroller (Utilities|Casting|CastToMrBoomAIController OwnerActor))
  (bind _asmr_boom_bp (Utilities|Casting|CastToMrBoomBP (Pawn|GetControlledPawn _asmr_boom_aicontroller)))
  (Variables|/Game/Blueprints/MrBOOM/MrBoomBP.MrBoomBP_C|SetMrBoomFired _asmr_boom_bp true)
  (Audio|PlaySound2D "/Game/Audio/MrBoomOpenfire.MrBoomOpenfire" 1.0 1.0 0.0 0 0)
  (Utilities|FireBulletsMacro (Math|Transform|MakeTransform (Transformation|GetSocketLocation (Variables|/Game/Blueprints/MrBOOM/MrBoomBP.MrBoomBP_C|GetMrBoomCannon _asmr_boom_bp) "Muzzle") (Math|Rotator|MakeRotator (.Roll (Math|Rotator|BreakRotator (Transformation|GetWorldRotation (Variables|/Game/Blueprints/MrBOOM/MrBoomBP.MrBoomBP_C|GetMrBoomCannon _asmr_boom_bp)))) (+ (.Pitch (Math|Rotator|BreakRotator (Transformation|GetWorldRotation (Variables|/Game/Blueprints/MrBOOM/MrBoomBP.MrBoomBP_C|GetMrBoomCannon _asmr_boom_bp)))) 1.8e+02) (.Yaw (Math|Rotator|BreakRotator (Transformation|GetWorldRotation (Variables|/Game/Blueprints/MrBOOM/MrBoomBP.MrBoomBP_C|GetMrBoomCannon _asmr_boom_bp)))))) (Math|Transform|MakeTransform (Transformation|GetSocketLocation (Variables|/Game/Blueprints/MrBOOM/MrBoomBP.MrBoomBP_C|GetMrBoomCannon _asmr_boom_bp) "Muzzle") (Math|Rotator|MakeRotator (.Roll (Math|Rotator|BreakRotator (Transformation|GetWorldRotation (Variables|/Game/Blueprints/MrBOOM/MrBoomBP.MrBoomBP_C|GetMrBoomCannon _asmr_boom_bp)))) (+ (.Pitch (Math|Rotator|BreakRotator (Transformation|GetWorldRotation (Variables|/Game/Blueprints/MrBOOM/MrBoomBP.MrBoomBP_C|GetMrBoomCannon _asmr_boom_bp)))) 1.8e+02) (.Yaw (Math|Rotator|BreakRotator (Transformation|GetWorldRotation (Variables|/Game/Blueprints/MrBOOM/MrBoomBP.MrBoomBP_C|GetMrBoomCannon _asmr_boom_bp)))))) (Math|Transform|MakeTransform (Transformation|GetSocketLocation (Variables|/Game/Blueprints/MrBOOM/MrBoomBP.MrBoomBP_C|GetMrBoomCannon _asmr_boom_bp) "Muzzle") (Math|Rotator|MakeRotator (.Roll (Math|Rotator|BreakRotator (Transformation|GetWorldRotation (Variables|/Game/Blueprints/MrBOOM/MrBoomBP.MrBoomBP_C|GetMrBoomCannon _asmr_boom_bp)))) (+ (.Pitch (Math|Rotator|BreakRotator (Transformation|GetWorldRotation (Variables|/Game/Blueprints/MrBOOM/MrBoomBP.MrBoomBP_C|GetMrBoomCannon _asmr_boom_bp)))) 1.8e+02) (.Yaw (Math|Rotator|BreakRotator (Transformation|GetWorldRotation (Variables|/Game/Blueprints/MrBOOM/MrBoomBP.MrBoomBP_C|GetMrBoomCannon _asmr_boom_bp)))))) (Math|Transform|MakeTransform (Transformation|GetSocketLocation (Variables|/Game/Blueprints/MrBOOM/MrBoomBP.MrBoomBP_C|GetMrBoomCannon _asmr_boom_bp) "Muzzle") (Math|Rotator|MakeRotator (.Roll (Math|Rotator|BreakRotator (Transformation|GetWorldRotation (Variables|/Game/Blueprints/MrBOOM/MrBoomBP.MrBoomBP_C|GetMrBoomCannon _asmr_boom_bp)))) (+ (.Pitch (Math|Rotator|BreakRotator (Transformation|GetWorldRotation (Variables|/Game/Blueprints/MrBOOM/MrBoomBP.MrBoomBP_C|GetMrBoomCannon _asmr_boom_bp)))) 1.8e+02) (.Yaw (Math|Rotator|BreakRotator (Transformation|GetWorldRotation (Variables|/Game/Blueprints/MrBOOM/MrBoomBP.MrBoomBP_C|GetMrBoomCannon _asmr_boom_bp)))))) (Math|Transform|MakeTransform (Transformation|GetSocketLocation (Variables|/Game/Blueprints/MrBOOM/MrBoomBP.MrBoomBP_C|GetMrBoomCannon _asmr_boom_bp) "Muzzle") (Math|Rotator|MakeRotator (.Roll (Math|Rotator|BreakRotator (Transformation|GetWorldRotation (Variables|/Game/Blueprints/MrBOOM/MrBoomBP.MrBoomBP_C|GetMrBoomCannon _asmr_boom_bp)))) (+ (.Pitch (Math|Rotator|BreakRotator (Transformation|GetWorldRotation (Variables|/Game/Blueprints/MrBOOM/MrBoomBP.MrBoomBP_C|GetMrBoomCannon _asmr_boom_bp)))) 1.8e+02) (.Yaw (Math|Rotator|BreakRotator (Transformation|GetWorldRotation (Variables|/Game/Blueprints/MrBOOM/MrBoomBP.MrBoomBP_C|GetMrBoomCannon _asmr_boom_bp)))))) (Math|Transform|MakeTransform (Transformation|GetSocketLocation (Variables|/Game/Blueprints/MrBOOM/MrBoomBP.MrBoomBP_C|GetMrBoomCannon _asmr_boom_bp) "Muzzle") (Math|Rotator|MakeRotator (.Roll (Math|Rotator|BreakRotator (Transformation|GetWorldRotation (Variables|/Game/Blueprints/MrBOOM/MrBoomBP.MrBoomBP_C|GetMrBoomCannon _asmr_boom_bp)))) (+ (.Pitch (Math|Rotator|BreakRotator (Transformation|GetWorldRotation (Variables|/Game/Blueprints/MrBOOM/MrBoomBP.MrBoomBP_C|GetMrBoomCannon _asmr_boom_bp)))) 1.8e+02) (.Yaw (Math|Rotator|BreakRotator (Transformation|GetWorldRotation (Variables|/Game/Blueprints/MrBOOM/MrBoomBP.MrBoomBP_C|GetMrBoomCannon _asmr_boom_bp)))))))
  (Class|BTFunctionLibrary|ClearBlackboardValue (Variables|Default|GetTarget))
  (AI|BehaviorTree|FinishExecute false))