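; Behavior tree task that aims the MrBoom enemy's cannon at the player unit stored in the Target blackboard key.
; It sets the cannon's world rotation to the look-at rotation computed from the player's location toward MrBoom, the reverse direction.
; It then plays a reload sound and finishes successfully after a short delay.
; A failed target cast only prints an error and never finishes the task.
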(event EventReceiveExecute
  (params (OwnerActor :type Actor%20Object%20Reference))
  (bind _asmr_boom_aicontroller (Utilities|Casting|CastToMrBoomAIController OwnerActor))
  (bind _asmr_boom_bp (Utilities|Casting|CastToMrBoomBP (Pawn|GetControlledPawn _asmr_boom_aicontroller)))
  (bind _asplayer_unit (Utilities|Casting|CastToPlayerUnit (AI|BehaviorTree|GetBlackboardValueasActor (Variables|Default|GetTarget)))
    (:then
      (Transformation|SetWorldRotation (Variables|/Game/Blueprints/MrBOOM/MrBoomBP.MrBoomBP_C|GetMrBoomCannon _asmr_boom_bp) (Math|Rotator|FindLookatRotation (Transformation|GetActorLocation _asplayer_unit) (Transformation|GetActorLocation _asmr_boom_bp)) false false)
      (Audio|PlaySound2D "/Game/Audio/MrBoomReload.MrBoomReload" 1.0 1.0 0.0 0 0)
      (Utilities|FlowControl|Delay 0.2)
      (AI|BehaviorTree|FinishExecute true))
    (:CastFailed
      (Development|PrintString "FAILED TO AQUIRE TARGET"))))