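; PlayerUnitController is the controller for a possessed PlayerUnit_BP, relaying move and shoot commands to that unit.
; Its MoveUnit and FireShot events cast the controlled pawn, then check that it has action points left and is not already moving.
; Only when both checks pass does it call the unit's Move with the given target or its ExecuteShot.
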(event Custom|MoveUnit
  (params (Target :type Vector))
  ;[1 1 1] Move Unit
  ;;[1 1 1] Validate Move
  (bind _asplayer_unit_bp (Utilities|Casting|CastToPlayerUnit_BP (Pawn|GetControlledPawn)))
  (bind _returnvalue (Class|BaseUnit|GetActionPoints _asplayer_unit_bp))
  (bind _returnvalue_2 (Class|BaseUnit|GetIsMoving _asplayer_unit_bp))
  (if (and (not _returnvalue_2) (> _returnvalue 0))
    (Default|Move _asplayer_unit_bp Target)))

(event Custom|FireShot
  (bind _asplayer_unit_bp (Utilities|Casting|CastToPlayerUnit_BP (Pawn|GetControlledPawn)))
  (bind _returnvalue (Class|BaseUnit|GetActionPoints _asplayer_unit_bp))
  (bind _returnvalue_2 (Class|BaseUnit|GetIsMoving _asplayer_unit_bp))
  (if (and (not _returnvalue_2) (> _returnvalue 0))
    (Default|ExecuteShot _asplayer_unit_bp)))

(fn ConstructionScript)