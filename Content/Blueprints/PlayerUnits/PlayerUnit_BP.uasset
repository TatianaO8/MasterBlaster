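; Player-controlled Paper2D sprite unit for an action-point, turn-based game, with move, shoot and click-to-select behavior.
; Clicking a unit with points left deactivates the current unit, updates the GameState and activates this one, snapping the camera to it.
; Move and shot events play audio, then call BeginMove and FireShot.
; Tick swaps run/idle flipbooks, follows movement via the PlayerController, and refreshes selection arrow and range rings from active state and remaining points.
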(event Custom|Activate
  ;[1 1 1] Switch and activate next unit
  (Utilities|FlowControl|Sequence
    (:then_0
      (bind _asmaster_blaster_pc_bp (Utilities|Casting|CastToMasterBlasterPC_BP (Game|GetPlayerController 0)))
      (Default|SnaptoUnit _asmaster_blaster_pc_bp self))
    (:then_1
      (bind _returnvalue (AddComponent|AddAudioComponent false))
      (Audio|Components|Audio|Play _returnvalue 0.0))
    (:then_2
      (Variables|Default|SetisActive true))))

(event Custom|De-activate
  (Variables|Default|SetisActive false))

(event Custom|Refresh
  (Utilities|DisplayRings))

(event Custom|UpdateAnimation
  (bind _sprite (Variables|Default|GetSprite))
  (bind _returnvalue (Class|BaseUnit|GetIsMoving))
  (if _returnvalue
    (Sprite|SetFlipbook _sprite "/Game/Sprites/PlayerSprites/Run/PlayerUnitRunAnimation.PlayerUnitRunAnimation")
    (else
      (Sprite|SetFlipbook _sprite "/Game/Sprites/PlayerSprites/Idle/PlayerUnitIdleAnimation.PlayerUnitIdleAnimation"))))

(event Custom|Move
  (params (Destination :type Vector))
  (Utilities|FlowControl|Sequence
    (:then_0
      (bind _returnvalue (AddComponent|AddAudioComponent false))
      (Audio|Components|Audio|Play _returnvalue 0.0))
    (:then_1
      (Class|BaseUnit|BeginMove Destination))))

(event Custom|ExecuteShot
  (bind _returnvalue (AddComponent|AddAudioComponent false))
  (Audio|Components|Audio|Play _returnvalue 0.0)
  (Class|BaseUnit|FireShot))

(event Custom|TakeDamage)

(event EventBeginPlay
  (Transformation|AttachComponentToComponent (Variables|Default|GetGunArm) (Variables|Default|GetSprite) "GunArm" "KeepRelative" "KeepRelative" "KeepRelative" true)
  ;[1 1 1] Initialize Health
  (bind _ashpbar (Utilities|Casting|CastToHPbar (UserInterface|GetUserWidgetObject (Variables|Default|GetHealthBar))))
  (bind _output_get (Variables|Default|SetHealthBarRef _ashpbar))
  (Variables|/Game/Blueprints/UI/HPbar.HPbar_C|SetCurrentHealth _output_get 1.0)
  (Variables|/Game/Blueprints/UI/HPbar.HPbar_C|SetMaxHealth _output_get 1.0))

(event EventTick
  (params (DeltaSeconds :type Float%20%28single-precision%29))
  (CallFunction|UpdateAnimation)
  (CallFunction|Refresh)
  (bind _returnvalue (Class|BaseUnit|GetIsMoving))
  (if _returnvalue
    (bind _asmaster_blaster_pc_bp (Utilities|Casting|CastToMasterBlasterPC_BP (Game|GetPlayerController 0)))
    (Default|FollowUnit _asmaster_blaster_pc_bp self)))

(event MouseInput|EventActorOnClicked
  (params (ButtonPressed :type Key%20Structure))
  ;[1 1 1] Unit direct picking
  (if (== ButtonPressed "LeftMouseButton")
    (bind _asmaster_blaster_game_state (Utilities|Casting|CastToMasterBlasterGameState (Game|GetGameState)))
    (bind _returnvalue (Class|BaseUnit|GetActionPoints))
    (if (> _returnvalue 0)
      (Utilities|FlowControl|Sequence
        (:then_0
          (bind _returnvalue_2 (Class|MasterBlasterGameState|GetActiveUnit _asmaster_blaster_game_state))
          (bind _asplayer_unit_bp (Utilities|Casting|CastToPlayerUnit_BP _returnvalue_2))
          (CallFunction|De-activate _asplayer_unit_bp))
        (:then_1
          (Class|MasterBlasterGameState|SetActiveUnit _asmaster_blaster_game_state (Variables|Default|GetteamIndex))
          (CallFunction|Activate)))
      (else
        (Development|PrintString "This unit is out of action points" true true "(R=1.000000,G=0.000000,B=0.000000,A=1.000000)")))))

(fn ConstructionScript)

(fn Display2AP
  (Rendering|SetVisibility (Variables|Default|GetSelectionArrow) true false)
  (Rendering|SetVisibility (Variables|Default|GetWalkRadius) true false)
  (Rendering|SetVisibility (Variables|Default|GetRunRadius) true false)
  (Rendering|SetVisibility (Variables|Default|GetWalk2Radius) false false))

(fn Display1AP
  (Rendering|SetVisibility (Variables|Default|GetWalk2Radius) true false)
  (Rendering|SetVisibility (Variables|Default|GetRunRadius) false false)
  (Rendering|SetVisibility (Variables|Default|GetSelectionArrow) true false)
  (Rendering|SetVisibility (Variables|Default|GetWalkRadius) false false))

(fn Display0AP
  (Rendering|SetVisibility (Variables|Default|GetSelectionArrow) false false)
  (Rendering|SetVisibility (Variables|Default|GetWalkRadius) false false)
  (Rendering|SetVisibility (Variables|Default|GetRunRadius) false false)
  (Rendering|SetVisibility (Variables|Default|GetWalk2Radius) false false))