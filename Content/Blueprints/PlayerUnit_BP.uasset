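; Player-controlled unit Blueprint that handles click selection and shows movement range by remaining action points.
; Left-clicking a unit with action points deactivates the game state's active unit and activates this one; otherwise it prints a warning.
; Activation plays a sound, refreshes the selection arrow and walk/run rings, and timeline-lerps the player pawn to the unit's X and Z, keeping its Y.
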(event Custom|Activate
  (bind _returnvalue (Game|Player|GetPlayerPawn 0))
  (bind _returnvalue_2 (Transformation|GetActorLocation))
  (bind _returnvalue_3 (Transformation|GetActorLocation _returnvalue))
  (bind (_x _y _z) (Math|Vector|BreakVector _returnvalue_2))
  ;[1 1 1] Switch and activate next unit
  (Utilities|FlowControl|Sequence
    (:then_0
      (Utilities|DisplayRings)
      (bind _returnvalue_4 (AddComponent|AddAudioComponent false))
      (Audio|Components|Audio|Play _returnvalue_4 0.0))
    (:then_1
      (bind _positioncurve (Timeline|MoveToActor%20Timeline PlayFromStart)
        (:Update
          (Transformation|SetActorLocation _returnvalue (Math|Vector|Lerp(Vector) _returnvalue_3 (Math|Vector|MakeVector _x (.Y (Math|Vector|BreakVector _returnvalue_3)) _z) _positioncurve) true false))))))

(event Custom|De-activate
  (Rendering|SetVisibility (Variables|Default|GetSelectionArrow) false false)
  (Rendering|SetVisibility (Variables|Default|GetWalkRadius) false false)
  (Rendering|SetVisibility (Variables|Default|GetRunRadius) false false)
  (Rendering|SetVisibility (Variables|Default|GetWalk2Radius) false false))

(event Custom|Refresh
  (Utilities|DisplayRings))

(event EventTick
  (params (DeltaSeconds :type Float%20%28single-precision%29)))

(event MouseInput|EventActorOnClicked
  (params (ButtonPressed :type Key%20Structure))
  ;[1 1 1] Unit direct picking
  (if (== ButtonPressed "LeftMouseButton")
    (bind _asmaster_blaster_game_state (Utilities|Casting|CastToMasterBlasterGameState (Game|GetGameState)))
    (bind _returnvalue (Class|BaseUnit|GetActionPoints))
    (if (> _returnvalue 0)
      (Utilities|FlowControl|Sequence
        (:then_0
          (bind _returnvalue_2 (Class|MasterBlasterGameState|GetActiveUnit _asmaster_blaster_game_state))
          (bind _asplayer_unit_bp (Utilities|Casting|CastToPlayerUnit_BP _returnvalue_2))
          (CallFunction|De-activate _asplayer_unit_bp))
        (:then_1
          (Class|MasterBlasterGameState|SetActiveUnit _asmaster_blaster_game_state (Variables|Default|GetteamIndex))
          (CallFunction|Activate)))
      (else
        (Development|PrintString "This unit is out of action points" true true "(R=1.000000,G=0.000000,B=0.000000,A=1.000000)")))))

(fn ConstructionScript)

(fn Display2AP
  (Rendering|SetVisibility (Variables|Default|GetSelectionArrow) true false)
  (Rendering|SetVisibility (Variables|Default|GetWalkRadius) true false)
  (Rendering|SetVisibility (Variables|Default|GetRunRadius) true false)
  (Rendering|SetVisibility (Variables|Default|GetWalk2Radius) false false))

(fn Display1AP
  (Rendering|SetVisibility (Variables|Default|GetWalk2Radius) true false)
  (Rendering|SetVisibility (Variables|Default|GetRunRadius) false false)
  (Rendering|SetVisibility (Variables|Default|GetSelectionArrow) true false)
  (Rendering|SetVisibility (Variables|Default|GetWalkRadius) false false))

(fn Display0AP
  (Rendering|SetVisibility (Variables|Default|GetSelectionArrow) false false)
  (Rendering|SetVisibility (Variables|Default|GetWalkRadius) false false)
  (Rendering|SetVisibility (Variables|Default|GetRunRadius) false false)
  (Rendering|SetVisibility (Variables|Default|GetWalk2Radius) false false))