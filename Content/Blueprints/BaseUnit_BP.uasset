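; BaseUnit_BP is a unit Blueprint that prints a debug greeting when clicked and holds pause and unpause functions.
; PauseGame pauses, creates the PauseMenu widget if it is invalid, shows it, and switches to UI-only input with the cursor visible.
; UnpauseGame resumes, removes all widgets and restores game-only input, keeping the cursor visible.
; Nothing in the Blueprint calls either function.
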(event MouseInput|EventActorOnClicked
  (params (ButtonPressed :type Key%20Structure))
  (Development|PrintString "Hello"))

(fn ConstructionScript)

(fn PauseGame
  (Game|SetGamePaused true)
  (Utilities|IsValid (Variables|Default|GetPauseMenu)
    (:Is%20Valid
      _)
    (:Is%20Not%20Valid
      (bind _returnvalue (UserInterface|CreateWidget "/Game/Blueprints/UI/PauseMenu.PauseMenu_C" (Game|GetPlayerController 0)))
      (Variables|Default|SetPauseMenu _returnvalue)))
  (UserInterface|Viewport|AddtoViewport (Variables|Default|GetPauseMenu) 0)
  (Input|SetInputModeUIOnly (Game|GetPlayerController 0) (Variables|Default|GetPauseMenu) "DoNotLock")
  (Variables|/Script/Engine.PlayerController|SetbShowMouseCursor (Game|GetPlayerController 0) true))

(fn UnpauseGame
  (bind _returnvalue (Game|GetPlayerController 0))
  (Game|SetGamePaused false)
  (Viewport|RemoveAllWidgets)
  (Input|SetInputModeGameOnly _returnvalue)
  (Variables|/Script/Engine.PlayerController|SetbShowMouseCursor _returnvalue true))