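; Basic enemy unit built on a Paper2D flipbook sprite, with a separate arm and a health bar widget.
; BeginPlay attaches the arm to the sprite's GunArm socket and caches the HPbar widget.
; Each tick switches between idle and run flipbooks based on movement and updates the bar with health divided by 100.
; RotateHealthBar orients the bar along the camera-to-bar direction but is not called within this Blueprint.
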(event Custom|UpdateAnimation
  (bind _sprite (Variables|Default|GetSprite))
  (bind _returnvalue (Class|BaseUnit|GetIsMoving))
  (if _returnvalue
    (Sprite|SetFlipbook _sprite "/Game/Sprites/EnemySprites/Run/EnemyUnitRunAnimation.EnemyUnitRunAnimation")
    (else
      (Sprite|SetFlipbook _sprite "/Game/Sprites/EnemySprites/Idle/EnemyIdleAnimation.EnemyIdleAnimation"))))

(event EventBeginPlay
  ;[1 1 1] Attatch arm
  (Transformation|AttachComponentToComponent (Variables|Default|GetArm) (Variables|Default|GetSprite) "GunArm" "KeepRelative" "KeepRelative" "KeepRelative" true)
  ;[1 1 1] Initialize Health
  (bind _ashpbar (Utilities|Casting|CastToHPbar (UserInterface|GetUserWidgetObject (Variables|Default|GetHealthBar))))
  (Variables|Default|SetHealthBarRef _ashpbar))

(event EventTick
  (params (DeltaSeconds :type Float%20%28single-precision%29))
  (CallFunction|UpdateAnimation)
  (bind _returnvalue (Class|BaseUnit|GetHealth))
  (Default|UpdateHealthBar (Variables|Default|GetHealthBarRef) (/ _returnvalue 1e+02)))

(fn ConstructionScript)

(fn RotateHealthBar
  (Transformation|SetWorldRotation (Variables|Default|GetHealthBar) (Math|Rotator|FindLookatRotation (Camera|GetCameraLocation (Game|GetPlayerCameraManager 0)) (Transformation|GetWorldLocation (Variables|Default|GetHealthBar))) false false))