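; Player controller for MasterBlaster that turns player input into commands for the active team unit held by MasterBlasterGameState.
; Move traces from the mouse cursor and passes only the hit's X to the unit, while Aim enables its raycast and Fire shoots.
; Cycling deactivates the current PlayerUnit_BP and activates the next, and Tick re-activates the active unit every frame.
; Pause opens the PauseMenu widget or resumes through it.
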(event EventBeginPlay
  ;[1 1 1] Select first unit on team when game starts
  (bind _asmaster_blaster_game_state (Utilities|Casting|CastToMasterBlasterGameState (Game|GetGameState)))
  (bind _returnvalue (Class|MasterBlasterGameState|GetActiveUnit _asmaster_blaster_game_state))
  (bind _asplayer_unit_bp (Utilities|Casting|CastToPlayerUnit_BP _returnvalue))
  (Default|Activate _asplayer_unit_bp))

(event EventTick
  (params (DeltaSeconds :type Float%20%28single-precision%29))
  (bind _asmaster_blaster_game_state (Utilities|Casting|CastToMasterBlasterGameState (Game|GetGameState)))
  (bind _returnvalue (Class|MasterBlasterGameState|GetActiveUnit _asmaster_blaster_game_state))
  (bind _asplayer_unit_bp (Utilities|Casting|CastToPlayerUnit_BP _returnvalue))
  (Default|Activate _asplayer_unit_bp))

(event Input|ActionEvents|InputActionPause
  (params (Key :type Key%20Structure))
  ;[1 1 1] Pause/Unpause logic
  (:Pressed
    (if (Game|IsGamePaused)
      (Default|Resume (stale _returnvalue))
      (else
        (bind _returnvalue (UserInterface|CreateWidget "/Game/Blueprints/PauseMenu.PauseMenu_C"))
        (UserInterface|Viewport|AddtoViewport _returnvalue 0)
        (Variables|/Script/Engine.PlayerController|SetbShowMouseCursor (Game|GetPlayerController 0) true)
        (Game|SetGamePaused true)))))

(event Input|ActionEvents|InputActionMove
  (params (Key :type Key%20Structure))
  (bind (_worldlocation _worlddirection) (Game|Player|ConvertMouseLocationToWorldSpace))
  (:Pressed
    (bind _asmaster_blaster_game_state (Utilities|Casting|CastToMasterBlasterGameState (Game|GetGameState)))
    (bind _returnvalue (Class|MasterBlasterGameState|GetActiveUnit _asmaster_blaster_game_state))
    (bind _outhit (Collision|LineTraceForObjects _worldlocation (+ _worlddirection (* (Math|Vector|GetForwardVector (Math|Conversions|RotationFromXVector _worlddirection)) 1e+06)) (Utilities|Array|MakeArray "ObjectTypeQuery1") false 0 "None"))
    (Class|BaseUnit|BeginMove _returnvalue (Math|Vector|MakeVector (.X (Math|Vector|BreakVector (.Location (Collision|BreakHitResult _outhit)))) 0.0 0.0))
    (bind _returnvalue_2 (AddComponent|AddAudioComponent false))
    (Audio|Components|Audio|Play _returnvalue_2 0.0)))

(event Input|ActionEvents|InputActionCycleUnit
  (params (Key :type Key%20Structure))
  ;[1 1 1] Unit Cycling
  (:Pressed
    (bind _asmaster_blaster_game_state (Utilities|Casting|CastToMasterBlasterGameState (Game|GetGameState))
      (:then
        (Utilities|FlowControl|Sequence
          (:then_0
            ;;[1 1 1] De-activate previous unit
            (bind _returnvalue (Class|MasterBlasterGameState|GetActiveUnit _asmaster_blaster_game_state))
            (bind _asplayer_unit_bp (Utilities|Casting|CastToPlayerUnit_BP _returnvalue))
            (Default|De-activate _asplayer_unit_bp))
          (:then_1
            ;;[1 1 1] Switch and activate next unit
            (Class|MasterBlasterGameState|CycleUnit _asmaster_blaster_game_state)
            (bind _returnvalue_2 (Class|MasterBlasterGameState|GetActiveUnit _asmaster_blaster_game_state))
            (bind _asplayer_unit_bp_2 (Utilities|Casting|CastToPlayerUnit_BP _returnvalue_2)
              (:then
                (Default|Activate _asplayer_unit_bp_2)
                (bind _returnvalue_3 (AddComponent|AddAudioComponent false))
                (Audio|Components|Audio|Play _returnvalue_3 0.0))
              (:CastFailed
                (Development|PrintString "You're fucked"))))))
      (:CastFailed
        (Development|PrintString "Bad game state")))))

(event Input|ActionEvents|InputActionAim
  (params (Key :type Key%20Structure))
  (:Pressed
    (bind _asmaster_blaster_game_state (Utilities|Casting|CastToMasterBlasterGameState (Game|GetGameState)))
    (bind _returnvalue (Class|MasterBlasterGameState|GetActiveUnit _asmaster_blaster_game_state))
    (Class|BaseUnit|EnableRaycast _returnvalue)))

(event Input|ActionEvents|InputActionFire
  (params (Key :type Key%20Structure))
  (:Pressed
    (bind _asmaster_blaster_game_state (Utilities|Casting|CastToMasterBlasterGameState (Game|GetGameState)))
    (bind _returnvalue (Class|MasterBlasterGameState|GetActiveUnit _asmaster_blaster_game_state))
    (Class|BaseUnit|FireShot _returnvalue)
    (bind _returnvalue_2 (AddComponent|AddAudioComponent false))
    (Audio|Components|Audio|Play _returnvalue_2 0.0)))

(fn ConstructionScript)